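; Super speed powerup that temporarily doubles the walk speed of the actor that activates it.
; OnActived stores that actor, sets its movement component's MaxWalkSpeed to twice GetMaxSpeed, which depends on movement mode, and prints the result on authority and non-authority alike.
; OnExpired sets it to half the then-current GetMaxSpeed if the actor is still valid, rather than restoring a saved value, then calls the parent's expiry.
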(event EventBeginPlay)

(event Collision|EventActorBeginOverlap
  (params (OtherActor :type Actor%20Object%20Reference)))

(event EventTick
  (params (DeltaSeconds :type Float%20%28single-precision%29)))

(event EventOnActived
  (params (OtherActor :type Actor%20Object%20Reference))
  (bind _returnvalue (Actor|GetComponentbyClass OtherActor "/Script/Engine.CharacterMovementComponent"))
  (bind _output_get (Variables|Default|SetOtherActor OtherActor))
  (bind _output_get_2 (Variables|/Script/Engine.CharacterMovementComponent|SetMaxWalkSpeed _returnvalue (* (Class|MovementComponent|GetMaxSpeed _returnvalue) 2.0)))
  (if (Utilities|Enum|Equal(Enum) (Networking|GetLocalRole _output_get) "ROLE_Authority")
    (Development|PrintString (Utilities|String|ToString(Float) _output_get_2))
    (else
      (Development|PrintString (Utilities|String|ToString(Float) _output_get_2)))))

(event EventOnExpired
  (bind _otheractor (Variables|Default|GetOtherActor))
  (bind _returnvalue (Actor|GetComponentbyClass _otheractor "/Script/Engine.CharacterMovementComponent"))
  (Utilities|IsValid _otheractor
    (:Is%20Valid
      (Variables|/Script/Engine.CharacterMovementComponent|SetMaxWalkSpeed _returnvalue (/ (Class|MovementComponent|GetMaxSpeed _returnvalue) 2.0)))
    (:Is%20Not%20Valid
      _))
  (|CallParentFunction))

(fn ConstructionScript)